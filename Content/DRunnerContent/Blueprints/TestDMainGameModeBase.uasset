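; Game mode for a runner level that ends the run and opens MainMap when all coins are gathered or the player loses.
; Tick compares gathered coins to the level maximum and otherwise, through a DoOnce, binds to every DPlayerBP's player-lost event.
; The lost handler flags the player as dead on the game instance.
; Both exit paths delete LoggedData.csv before the level change.
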(event Custom|CustomEvent
  (bind _asdgame_instance_bp (Utilities|Casting|CastToDGameInstanceBP (Game|GetGameInstance)))
  (Variables|/Script/DRunner.DGameInstance|SetIsPlayerDead _asdgame_instance_bp true)
  (Class|TestFunctions|DeleteFileifExists "" "LoggedData.csv")
  (Game|OpenLevel(byName) "MainMap"))

(event EventTick
  (params (DeltaSeconds :type Float%20%28single-precision%29))
  (if (== (Math|Float|Truncate (Variables|Default|GetCurrentGatheredCoins)) (Variables|Default|GetMaxCoinsOnLevel))
    (Class|TestFunctions|DeleteFileifExists "" "LoggedData.csv")
    (Game|OpenLevel(byName) "MainMap")
    (else
      (Utilities|FlowControl|DoOnce false
        (:Completed
          (bind _outactors (Actor|GetAllActorsOfClass "/Game/DRunnerContent/Blueprints/DPlayerBP.DPlayerBP_C"))
          (for _array_element _outactors
            (EventDispatchers|BindEventtoOnEventPlayerLost _array_element (delegate Custom|CustomEvent))))))))

(fn ConstructionScript)