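; Game mode for DRunner that ends the level on either win or player loss by opening the EndScreen level.
; Tick compares gathered coins with the level's truncated maximum and, until they match, uses a DoOnce to bind each DPlayerBP's player-lost event.
; The loss handler flags IsPlayerDead on the game instance before switching levels.
; A LoadAndSaveBP widget creation chain exists but is unconnected.
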(event Custom|CustomEvent
  (bind _asdgame_instance_bp (Utilities|Casting|CastToDGameInstanceBP (Game|GetGameInstance)))
  (Variables|/Script/DRunner.DGameInstance|SetIsPlayerDead _asdgame_instance_bp true)
  (Game|OpenLevel(byName) "EndScreen"))

(event EventBeginPlay)

(event EventTick
  (params (DeltaSeconds :type Float%20%28single-precision%29))
  (if (== (Variables|Default|GetCurrentGatheredCoins) (Math|Float|Truncate (Variables|Default|GetMaxCoinsOnLevel)))
    (Game|OpenLevel(byName) "EndScreen")
    (else
      (Utilities|FlowControl|DoOnce false
        (:Completed
          (bind _outactors (Actor|GetAllActorsOfClass "/Game/DRunnerContent/Blueprints/DPlayerBP.DPlayerBP_C"))
          (for _array_element _outactors
            (EventDispatchers|BindEventtoOnEventPlayerLost _array_element (delegate Custom|CustomEvent))
            (Utilities|FlowControl|DoOnce false
              (:Completed
                (if true
                  _)))))))))

(fn ConstructionScript)