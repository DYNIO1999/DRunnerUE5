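; Virtusphere controller Blueprint that drives player pawn movement from the velocity in the current pose event.
; Each tick it scales the X and Y velocities, normalizes them against the character's max walk speed and feeds them as movement input along the pawn's right and forward vectors.
; It also prints the game instance's platform type and an angle value every tick for debugging.
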(event EventTick
  (params (DeltaSeconds :type Float%20%28single-precision%29))
  (bind _returnvalue (Game|Player|GetPlayerPawn 0))
  (bind _currentposeevent (Variables|Default|GetCurrentPoseEvent))
  (bind _returnvalue_2 (Actor|GetComponentbyClass _returnvalue "/Script/Engine.CharacterMovementComponent"))
  (bind _maxwalkspeed (Variables|/Script/Engine.CharacterMovementComponent|GetMaxWalkSpeed _returnvalue_2))
  (Pawn|Input|AddMovementInput _returnvalue (* (+ (* (Transformation|GetActorRightVector _returnvalue) (Math|Float|NormalizetoRange (* (.velocityvectorx _currentposeevent) 1e+02) 0.0 _maxwalkspeed)) (* (Transformation|GetActorForwardVector _returnvalue) (Math|Float|NormalizetoRange (* (.velocityvectory _currentposeevent) 1e+02) 0.0 _maxwalkspeed))) 1.0) 1.0 false)
  (Development|PrintString (Utilities|String|EnumtoString (Variables|/Script/DRunner.DGameInstance|GetCurrentPlatformType (Variables|Default|GetDGameInstance))))
  (Development|PrintString (Utilities|String|ToString(Float) (Variables|Default|GetAngle))))

(fn ConstructionScript)