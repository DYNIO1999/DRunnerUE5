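; Virtusphere control Blueprint that connects to a local device server and turns sphere motion into player pawn movement.
; On connect it requests pose, motor and controller updates, and disconnects at EndPlay.
; Tick scales pose velocity against max walk speed and applies it along the pawn's right and forward vectors.
; Controller states go to the game instance, as does the motor state array after every four inserts, skipping the event that triggers publishing.
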(event EventBeginPlay
  (Class|VirtuSphereController|Connect "127.0.0.1" 4445))

(event EventOnMotorState
  (params (event :type Motor%20State%20Event%20Structure))
  (if (== (Variables|Default|Getindex) 4)
    (Variables|Default|Setindex 0)
    (Variables|/Script/DRunner.DGameInstance|SetCurrentMotorStateEvent (Variables|Default|GetDGameInstanceRef) (Variables|Default|GetMotorStates))
    (else
      (Utilities|Array|Insert (Variables|Default|GetMotorStates) event (Variables|Default|Getindex))
      (bind _result (Math|Integer|IncrementInt (Variables|Default|Getindex))
        (:%20%20
          (Variables|Default|Setindex _result))))))

(event EventTick
  (params (DeltaSeconds :type Float%20%28single-precision%29))
  (bind _returnvalue (Game|Player|GetPlayerPawn 0))
  (bind _movementinput (Variables|Default|GetMovementInput))
  (bind _returnvalue_2 (Actor|GetComponentbyClass _returnvalue "/Script/Engine.CharacterMovementComponent"))
  (bind _maxwalkspeed (Variables|/Script/Engine.CharacterMovementComponent|GetMaxWalkSpeed _returnvalue_2))
  (Pawn|Input|AddMovementInput _returnvalue (* (+ (* (Transformation|GetActorRightVector _returnvalue) (Math|Float|NormalizetoRange (* (.x _movementinput) 1e+02) 0.0 _maxwalkspeed)) (* (Transformation|GetActorForwardVector _returnvalue) (Math|Float|NormalizetoRange (* (.y _movementinput) 1e+02) 0.0 _maxwalkspeed))) 1.0) 1.0 false)
  (bind _asdgame_instance_bp (Utilities|Casting|CastToDGameInstanceBP (Game|GetGameInstance)))
  (Variables|Default|SetDGameInstanceRef _asdgame_instance_bp))

(event EventEndPlay
  (params (EndPlayReason :type EEndPlayReason%20Enum :default "Destroyed"))
  (Class|VirtuSphereController|Disconnect))

(event EventOnConnected
  (Class|VirtuSphereController|RequestSpherePoseUpdates 10)
  (Class|VirtuSphereController|RequestMotorStateUpdates 20)
  (Class|VirtuSphereController|RequestControllerStateUpdates 20))

(event EventOnSpherePose
  (params (event :type Sphere%20Pose%20Event%20Structure))
  (Variables|Default|SetMovementInput (Math|Vector|MakeVector (.velocityvectorx event) (.velocityvectory event) (.velocityvectorz event))))

(event EventOnControllerState
  (params (event :type Controller%20State%20Event%20Structure))
  (Variables|/Script/DRunner.DGameInstance|SetCurrentControllerStateEvent (Variables|Default|GetDGameInstanceRef) event))

(fn ConstructionScript)