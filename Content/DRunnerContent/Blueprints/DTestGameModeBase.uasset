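; DTestGameModeBase is a game mode Blueprint that restarts the current level when the player loses.
; On Tick, behind a DoOnce, it finds every DPlayerBP actor and binds a custom event to its OnEventPlayerLost dispatcher.
; That event sets IsPlayerDead on DGameInstanceBP, so the flag outlives the reload, then reopens the current level by name.
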(event Custom|CustomEvent
  (bind _asdgame_instance_bp (Utilities|Casting|CastToDGameInstanceBP (Game|GetGameInstance)))
  (Variables|/Script/DRunner.DGameInstance|SetIsPlayerDead _asdgame_instance_bp true)
  (bind _returnvalue (Game|GetCurrentLevelName true))
  (Game|OpenLevel(byName) (Utilities|String|StringToName _returnvalue)))

(event EventTick
  (params (DeltaSeconds :type Float%20%28single-precision%29))
  (Utilities|FlowControl|DoOnce false
    (:Completed
      (bind _outactors (Actor|GetAllActorsOfClass "/Game/DRunnerContent/Blueprints/DPlayerBP.DPlayerBP_C"))
      (for _array_element _outactors
        (EventDispatchers|BindEventtoOnEventPlayerLost _array_element (delegate Custom|CustomEvent))))))

(fn ConstructionScript)